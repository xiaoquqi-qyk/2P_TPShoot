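; BP_砖头 is a thrown brick projectile, filed under AI weapons, that damages either of two players.
; On BeginPlay it sets a short lifespan and launches the brick mesh with a mass-scaled impulse opposite its Arrow's forward direction.
; On hit, it applies damage once if the other actor is player pawn 0 or 1, and destroys itself.
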(event OnComponentHit(砖头)
  (params (HitComponent :type Primitive%20Component%20Object%20Reference) (OtherActor :type Actor%20Object%20Reference) (OtherComp :type Primitive%20Component%20Object%20Reference) (NormalImpulse :type Vector :default "0, 0, 0") (Hit :type Hit%20Result%20Structure%20%28by%20ref%29))
  ;[1 1 1] Compare who he hits
  (if (or (== OtherActor (Game|Player|GetPlayerPawn 0)) (== OtherActor (Game|Player|GetPlayerPawn 1)))
    (Utilities|FlowControl|DoOnce false
      (:Completed
        (Game|Damage|ApplyDamage OtherActor 1.0 0 0))))
  (Actor|DestroyActor))

(event EventBeginPlay
  (bind _砖头 (Variables|Default|Get砖头))
  (bind _arrow (Variables|Default|GetArrow))
  (bind _returnvalue (Transformation|GetWorldTransform _arrow))
  ;[1 1 1] 发射砖头和设置砖头生命周期
  (Utilities|IsValid self
    (:Is%20Valid
      (Actor|SetLifeSpan self 2.0)
      (Physics|AddImpulseatLocation _砖头 (* (Math|Vector|NegateVector (Math|Vector|GetForwardVector (.rotation _returnvalue))) (* (Physics|GetMass _砖头) 2e+03)) (.location _returnvalue) "None"))))

(fn ConstructionScript)